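; BP_武器 (Weapon) is a gun Blueprint that handles automatic firing and magazine reloading.
; Holding the 攻擊 (Attack) input runs a Delay-paced loop while ammo remains, spawning BP_子彈 bullets and a muzzle particle at the weapon mesh's bullet socket.
; Each shot decrements the current ammo count.
; The custom event 換彈夾 (Reload) refills the magazine from total ammo, capped by what remains.
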(event Custom|換彈夾
  ;[1 1 1] 計算要補充的子彈數
  (Variables|Default|Set需補充的子彈數量 (- (Variables|Default|Get彈夾尺寸) (Variables|Default|Get目前子彈數量)))
  ;[1 1 1] 判斷子彈夠不夠
  (if (>= (Variables|Default|Get子彈總數) (Variables|Default|Get需補充的子彈數量))
    _
    (else
      ;[1 1 1] 總數<彈夾數
      (Variables|Default|Set需補充的子彈數量 (Variables|Default|Get子彈總數))))
  ;[1 1 1] 目前子彈及總數更新
  (Variables|Default|Set目前子彈數量 (+ (Variables|Default|Get目前子彈數量) (Variables|Default|Get需補充的子彈數量)))
  (Variables|Default|Set子彈總數 (- (Variables|Default|Get子彈總數) (Variables|Default|Get需補充的子彈數量))))

(event Input|ActionEvents|InputAction攻擊
  (params (Key :type Key%20Structure :default "None"))
  (bind _武器模型 (Variables|Default|Get武器模型))
  (bind _returnvalue (Transformation|GetSocketRotation _武器模型 "子彈插槽"))
  ;[1 1 1] 開槍
  (:Pressed
    (Variables|Default|Set開槍中 true)
    (if (and (Variables|Default|Get開槍中) (> (Variables|Default|Get目前子彈數量) 0)) :!label _label ; 子彈數大於1
      (Game|SpawnActorfromClass "/Game/BP/BP_子彈.BP_子彈_C" (Transformation|GetSocketTransform (Variables|Default|Get武器模型) "子彈插槽" "RTS_World") "Undefined" 0 0) ; 生成子彈藍圖
      (Effects|SpawnEmitteratLocation "/Game/InfinityBladeEffects/Effects/FX_Skill_Whirlwind/P_Whirlwind_Default_Start_01.P_Whirlwind_Default_Start_01" (Transformation|GetSocketLocation _武器模型 "子彈插槽") (Math|Rotator|MakeRotator (.roll _returnvalue) (.pitch _returnvalue) (+ (.yaw _returnvalue) 9e+01)) "0.100000,0.100000,0.100000")
      (Variables|Default|Set目前子彈數量 (- (Variables|Default|Get目前子彈數量) 1)) ; 開槍扣子彈
      (Utilities|FlowControl|Delay (Variables|Default|Get開槍間隔))
      (goto _label)))
  (:Released
    (Variables|Default|Set開槍中 false)))

(fn ConstructionScript)