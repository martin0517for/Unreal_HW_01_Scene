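; Game mode Blueprint that runs a minutes-and-seconds countdown and pauses the game when time runs out.
; On BeginPlay it counts actors tagged "怪物" (monster) and stores the total as the required kill count.
; Tick feeds a one-second Delay that throttles the countdown, decrementing seconds and borrowing from minutes when seconds drop below zero.
; The kill count is only set here, not checked.
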(event EventTick
  (params (DeltaSeconds :type Float%20%28single-precision%29))
  ;[1 1 1] 倒數系統
  ;;[1 1 1] 每秒減1
  (Utilities|FlowControl|Delay 1.0) ; 延遲
  (bind _output_get (Variables|Default|Set秒 (- (Variables|Default|Get秒) 1)))
  ;;[1 1 1] 判斷秒數是否低於0 並設秒為59
  (if (< _output_get 0) ; 判斷
    (Variables|Default|Set秒 59)
    ;;[1 1 1] 檢查分 並把分-1
    (if (> (Variables|Default|Get分) 0)
      (Variables|Default|Set分 (- (Variables|Default|Get分) 1))
      (else
        ;;[1 1 1] 時間結束暫停遊戲
        (if (== (Variables|Default|Get秒) 59)
          (Variables|Default|Set秒 0)
          (Game|SetGamePaused true))))))

(event EventBeginPlay
  (bind _outactors (Actor|GetAllActorswithTag "怪物"))
  (Variables|Default|Set需要擊殺的怪物數量 (Utilities|Array|Length _outactors)))

(fn ConstructionScript)